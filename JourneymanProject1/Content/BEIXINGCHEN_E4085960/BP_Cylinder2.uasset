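; Actor that animates a cylinder between two marker points while pitching a scene component, apparently as a moving level prop.
; On BeginPlay, ReverseOrder selects one of two timelines that lerp the Cylinder's relative location from Point1 to Point2.
; Each movement update also calls Play on a shared rotation timeline, which drives the Scene component's relative pitch.
; Overlap and Tick events are unused.
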(event EventBeginPlay
  (if (Variables|Default|GetReverseOrder)
    (bind _新建轨道_0 (Timeline|Timeline Play)
      (:Update
        (Transformation|SetRelativeLocation (Variables|Default|GetCylinder) (Math|Vector|Lerp(Vector) (Variables|/Script/Engine.SceneComponent|GetRelativeLocation (Variables|Default|GetPoint1)) (Variables|/Script/Engine.SceneComponent|GetRelativeLocation (Variables|Default|GetPoint2)) _新建轨道_0) false false)
        (bind _新建轨道_0_2 (Timeline|时间轴_0 Play)
          (:Update
            (Transformation|SetRelativeRotation (Variables|Default|GetScene) (Math|Rotator|MakeRotator 0.0 _新建轨道_0_2 0.0) false false)))))
    (else
      (bind _新建轨道_0_3 (Timeline|时间轴 Play)
        (:Update
          (Transformation|SetRelativeLocation (Variables|Default|GetCylinder) (Math|Vector|Lerp(Vector) (Variables|/Script/Engine.SceneComponent|GetRelativeLocation (Variables|Default|GetPoint1)) (Variables|/Script/Engine.SceneComponent|GetRelativeLocation (Variables|Default|GetPoint2)) _新建轨道_0_3) false false)
          (Timeline|时间轴_0 Play))))))

(event Collision|EventActorBeginOverlap
  (params (OtherActor :type Actor%20Object%20Reference)))

(event EventTick
  (params (DeltaSeconds :type Float%20%28single-precision%29)))

(fn ConstructionScript)