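; Thrown cog projectile that spins out from its owner, deals heavy attacks while moving, then returns to its CompanionCog.
; Timers stop its flight, enable Pawn-blocking collision and trigger the return; hitting another actor also stops it.
; The owner leaving the JumpOff overlap volume triggers an early return.
; Returning disables collision and interpolates toward the CompanionCog's transform on Tick, destroying the actor on arrival or if the companion is invalid.
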(event OnComponentEndOverlap(JumpOff)
  (params (OverlappedComponent :type Primitive%20Component%20Object%20Reference) (OtherActor :type Actor%20Object%20Reference) (OtherComp :type Primitive%20Component%20Object%20Reference) (OtherBodyIndex :type Integer))
  (if (== OtherActor (Variables|Refs|GetOwningActor))
    (CallFunction|Despawn)))

(event OnComponentHit(Collision)
  (params (HitComponent :type Primitive%20Component%20Object%20Reference) (OtherActor :type Actor%20Object%20Reference) (OtherComp :type Primitive%20Component%20Object%20Reference) (NormalImpulse :type Vector :default "0, 0, 0") (Hit :type Hit%20Result%20Structure%20%28by%20ref%29))
  (if (!= OtherActor (Variables|Refs|GetOwningActor))
    (CallFunction|StopMovement)))

(event Custom|HitDetect
  (Default|HeavyAttack (Variables|Default|GetC_Attack) (Variables|/Script/Engine.BoxComponent|GetBoxExtent (Variables|Default|GetJump%20Off))))

(event Custom|Start%20Movement
  (params (Direction :type Vector) (Speed :type Float%20%28double-precision%29))
  ;[0.15 0.15 0.15 0.5] Stop / Start Movement
  (Variables|/Script/Engine.MovementComponent|SetVelocity (Variables|Default|GetProjectileMovement) (* Direction Speed))
  (Variables|Kinematics|SetMoving true))

(event Custom|Despawn
  (CallFunction|DisableCollision)
  (Variables|Kinematics|SetReturning true)
  (Variables|Kinematics|SetMoving true))

(event Custom|Throw%20Cog
  (params (Direction :type Vector) (Speed :type Float%20%28double-precision%29))
  (CallFunction|DisableCollision)
  (CallFunction|StartMovement Direction Speed)
  (Utilities|Time|SetTimerbyEvent (delegate Custom|Stop%20Movement) (Variables|Lifetime|GetStop%20Movement%20At))
  (Utilities|Time|SetTimerbyEvent (delegate Custom|Enable%20Collision) (Variables|Lifetime|GetEnable%20Collision%20At))
  (Utilities|Time|SetTimerbyEvent (delegate Custom|Despawn) (Variables|Lifetime|GetDespawn%20At)))

(event Custom|Disable%20Collision
  (bind _collision (Variables|Default|GetCollision))
  ;[0.15 0.15 0.15 0.5] Collision Setters
  (Variables|/Script/Engine.PrimitiveComponent|SetbGenerateOverlapEvents (Variables|Default|GetJump%20Off) false)
  (Variables|/Script/Engine.PrimitiveComponent|SetbGenerateOverlapEvents _collision false)
  (Collision|SetCollisionResponsetoChannel _collision "ECC_Pawn" "ECR_Ignore"))

(event Custom|Enable%20Collision
  (bind _collision (Variables|Default|GetCollision))
  ;[0.15 0.15 0.15 0.5] Collision Setters
  (Variables|/Script/Engine.PrimitiveComponent|SetbGenerateOverlapEvents (Variables|Default|GetJump%20Off) true)
  (Variables|/Script/Engine.PrimitiveComponent|SetbGenerateOverlapEvents _collision true)
  (Collision|SetCollisionResponsetoChannel _collision "ECC_Pawn" "ECR_Block"))

(event Custom|Stop%20Movement
  ;[0.15 0.15 0.15 0.5] Stop / Start Movement
  (Components|Movement|StopMovementImmediately (Variables|Default|GetProjectileMovement))
  (Variables|Kinematics|SetMoving false))

(event EventBeginPlay
  (CallFunction|ThrowCog (Variables|Kinematics|GetDirection) (Variables|Kinematics|GetSpeed)))

(event EventTick
  (params (DeltaSeconds :type Float%20%28single-precision%29))
  (if (Variables|Kinematics|GetReturning)
    (if (CallFunction|ResetPosition DeltaSeconds)
      (Actor|DestroyActor)
      (else
        (CallFunction|HitDetect)))
    (else
      (Transformation|AddRelativeRotation (Variables|Default|GetMesh) (Math|Rotator|MakeRotator 0.0 0.0 (* DeltaSeconds (Variables|Kinematics|GetRotationRate))) false false)
      (if (Variables|Kinematics|GetMoving)
        (CallFunction|HitDetect)))))

(fn ConstructionScript)

(fn ResetPosition
  (params (Delta :type Float%20%28double-precision%29))
  (bind _returnvalue (Transformation|GetActorLocation))
  (bind _companioncog (Variables|Refs|GetCompanionCog))
  (bind _socketlocation (Default|GetCogTransform _companioncog))
  (Utilities|IsValid _companioncog
    (:Is%20Valid
      (Utilities|FlowControl|Sequence
        (:then_0
          (Transformation|SetActorRotation (Class|KismetMathLibrary|RInterptoConstant (Transformation|GetActorRotation) (.rotation _socketlocation) Delta 1.5e+03)))
        (:then_1
          (Transformation|SetActorLocation (Math|Interpolation|VInterptoConstant _returnvalue (.location _socketlocation) Delta 1.5e+03) false false)
          (return (<= (Math|Vector|Distance(Vector) _returnvalue (.location _socketlocation)) 1e+01)))))
    (:Is%20Not%20Valid
      (return true))))

(fn IsStationary
  (return (<= (Math|Vector|VectorLength (Variables|/Script/Engine.MovementComponent|GetVelocity (Variables|Default|GetProjectileMovement))) 0.01)))