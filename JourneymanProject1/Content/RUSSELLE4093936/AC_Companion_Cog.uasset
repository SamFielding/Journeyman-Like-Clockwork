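; Companion cog component that gives the player a cog mesh and its related roll dash and spin attack abilities.
; On BeginPlay it spawns a StaticMeshActor, sets it up as a collision-free movable cog, and attaches it to player 0's CompanionCogSocket.
; It then adds both skill components to that character.
; Destroying the cog is faked by disabling and hiding the mesh, leaving the actor and abilities in place.
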(event Custom|DestroyCompanionCog
  ;[0.15 0.15 0.15 0.5] Faux Destroy Self
  (Variables|Default|SetEnabled false)
  (CallFunction|SetVisible false))

(event Custom|SetVisible
  (params (Visible :type Boolean))
  ;[0.15 0.15 0.15 0.5] Hide the Cog Mesh
  (bind _output_get (Variables|Default|SetEnabled Visible))
  (Rendering|SetVisibility (Variables|/Script/Engine.StaticMeshActor|GetStaticMeshComponent (Variables|Default|GetStaticMesh)) _output_get true))

(event EventBeginPlay
  (bind _returnvalue (Game|GetPlayerCharacter 0))
  (bind _returnvalue_2 (Game|GetPlayerCharacter 0))
  ;[0.15 0.15 0.15 0.5] Create the static mesh and attach it to the player
  (bind _returnvalue_3 (Game|SpawnActorfromClass "/Script/Engine.StaticMeshActor" (Transformation|GetActorTransform _returnvalue) "Undefined" "MultiplyWithRoot" _returnvalue 0))
  ;[0.15 0.15 0.15 0.5] Update the now created static mesh
  (Variables|Default|SetStaticMesh _returnvalue_3)
  (CallFunction|SetStaticMesh)
  ;[0.15 0.15 0.15 0.5] Attach the cog to the player mesh, in the specific cog slot. (CompanionCogSocket)
  (Transformation|AttachComponentToComponent (Variables|Default|GetStaticMesh) (Variables|/Script/Engine.Character|GetMesh _returnvalue) "CompanionCogSocket" "SnapToTarget" "SnapToTarget" "KeepWorld" true)
  ;[0.15 0.15 0.15 0.5] Ensure that the cog is rotated correctly on the player
  (Transformation|SetRelativeRotation (Variables|/Script/Engine.Actor|GetRootComponent (Variables|Default|GetStaticMesh)) "90.000000,0.000000,0.000000" false false)
  ;[0.15 0.15 0.15 0.5] Attach Skill Abilities to Player
  (Game|AddComponentbyClass _returnvalue_2 "/Game/BEIXINGCHEN_E4085960/BXC-CharactersSkills/BXC_AC_CogRollDash.BXC_AC_CogRollDash_C")
  (Game|AddComponentbyClass _returnvalue_2 "/Game/BEIXINGCHEN_E4085960/BXC-CharactersSkills/BXC_AC_CogSpinAttack.BXC_AC_CogSpinAttack_C"))

(fn SetStaticMesh
  (bind _staticmesh (Variables|Default|GetStaticMesh))
  (bind _staticmeshcomponent (Variables|/Script/Engine.StaticMeshActor|GetStaticMeshComponent _staticmesh))
  (Utilities|IsValid _staticmesh
    (:Is%20Valid
      ;[0.15 0.15 0.15 0.5] Ensure that the object will not fall through the world, player or have any wacky interactions
      (Collision|SetCollisionEnabled _staticmeshcomponent "NoCollision")
      ;[0.15 0.15 0.15 0.5] Allow the object to be moved with the player
      (Transformation|SetMobility (Variables|Default|GetStaticMesh) "Movable")
      ;[0.15 0.15 0.15 0.5] Set the static mesh and it's material
      (Components|StaticMesh|SetStaticMesh _staticmeshcomponent "/Game/CUNNINGHAME4080343/AC_ART_BO_Objects/AC_SM_BO_Cog_2m.AC_SM_BO_Cog_2m")
      (Rendering|Material|SetMaterial _staticmeshcomponent 0 "/Game/RUSSELLE4093936/M_Cog_Test.M_Cog_Test")
      (return))))