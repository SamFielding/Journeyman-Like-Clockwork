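; BP_CogSwitch is a cog that turns while the third-person player spins inside its trigger sphere.
; Sphere overlap stores the player and starts a looping timer, which is cleared when the player leaves.
; Each timer step checks the player's IsSpinning flag and adds local roll to the mesh, scaled by speed and interval, avoiding Tick.
; Despite the switch name, no mechanism activation is wired up.
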(event OnComponentBeginOverlap(Sphere)
  (params (OverlappedComponent :type Primitive%20Component%20Object%20Reference) (OtherActor :type Actor%20Object%20Reference) (OtherComp :type Primitive%20Component%20Object%20Reference) (OtherBodyIndex :type Integer) (bFromSweep :type Boolean) (SweepResult :type Hit%20Result%20Structure%20%28by%20ref%29))
  (bind _asbp_third_person_character (Utilities|Casting|CastToBP_ThirdPersonCharacter OtherActor))
  (Variables|Default|SetPlayerRef _asbp_third_person_character)
  (Variables|Default|SetIsPlayerInside true)
  (CallFunction|StartRotate))

(event OnComponentEndOverlap(Sphere)
  (params (OverlappedComponent :type Primitive%20Component%20Object%20Reference) (OtherActor :type Actor%20Object%20Reference) (OtherComp :type Primitive%20Component%20Object%20Reference) (OtherBodyIndex :type Integer))
  (Utilities|Casting|CastToBP_ThirdPersonCharacter OtherActor)
  (Variables|Default|SetIsPlayerInside false)
  (CallFunction|StopRotate))

(event Custom|RotateStep
  (if (and (Variables|Default|GetIsPlayerInside) (Variables|/Game/ThirdPerson/Blueprints/BP_ThirdPersonCharacter.BP_ThirdPersonCharacter_C|GetIsSpinning (Variables|Default|GetPlayerRef)))
    (Transformation|AddLocalRotation (Variables|Default|GetStaticMesh) (Math|Rotator|MakeRotator (* (Variables|Default|GetRotationSpeed) (Variables|Default|GetRotateInterval)) 0.0 0.0) false false)))

(event Custom|StartRotate
  (if (not (Utilities|Time|IsTimerActivebyHandle (Variables|Default|GetRotateTimerHandle)))
    (bind _returnvalue (Utilities|Time|SetTimerbyEvent (delegate Custom|RotateStep) (Variables|Default|GetRotateInterval) true))
    ;[0.15 0.15 0.15 0.5] Then connect the event that triggers the mechanism activation.
    (Variables|Default|SetRotateTimerHandle _returnvalue)))

(event Custom|StopRotate
  (Utilities|Time|ClearandInvalidateTimerbyHandle (Variables|Default|GetRotateTimerHandle)))

(event EventBeginPlay)

(event Collision|EventActorBeginOverlap
  (params (OtherActor :type Actor%20Object%20Reference)))

(event EventTick
  (params (DeltaSeconds :type Float%20%28single-precision%29)))

(fn ConstructionScript)