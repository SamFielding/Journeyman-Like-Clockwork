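; Actor component that stores a checkpoint for its owning actor and returns the actor to it on respawn.
; BeginPlay records the owner's starting location as the default checkpoint, and SetCheckpoint overwrites it with the value passed in.
; Respawn teleports the owner to the stored location without sweeping, setting only location and leaving rotation untouched.
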(event EventSetCheckpoint
  (params (Checkpoint%20Transform :type Vector :default "0, 0, 0"))
  (Variables|Default|SetCheckpoint Checkpoint%20Transform))

(event EventRespawn
  (bind _returnvalue (Components|GetOwner))
  (Utilities|IsValid _returnvalue
    (:Is%20Valid
      (Transformation|SetActorLocation _returnvalue (Variables|Default|GetCheckpoint) false true))))

(event EventBeginPlay
  (bind _returnvalue (Components|GetOwner))
  (Utilities|IsValid _returnvalue
    (:Is%20Valid
      (Variables|Default|SetCheckpoint (Transformation|GetActorLocation _returnvalue)))))