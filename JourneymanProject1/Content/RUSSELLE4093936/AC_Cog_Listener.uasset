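; AC_Cog_Listener is a component that relays state and speed changes from an attached cog.
; On BeginPlay it binds to the attached cog's update and speed-change dispatchers, if the cog is valid, and forwards each event through its own dispatchers.
; A LockCog event sets the cog to a fixed state, sends it an update message with that state, and prints a debug string.
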(event Custom|Cog%20Updated
  (params (NewState :type E_State%20Enum :default "NewEnumerator0"))
  (Default|CallCogUpdated NewState))

(event Custom|CogSpeedChanged
  (params (Speed :type Float%20%28double-precision%29))
  (Default|CallCogSpeedUpdated Speed))

(event Custom|LockCog
  (Default|SetCogState (Variables|Default|GetAttachedCog) "NewEnumerator1")
  (Class|BPICogCommunication|CogUpdated(Message) (Variables|Default|GetAttachedCog) 0 "NewEnumerator1")
  (Development|PrintString "CogLockedCalled"))

(event EventBeginPlay
  (bind _attachedcog (Variables|Default|GetAttachedCog))
  (Utilities|IsValid _attachedcog
    (:Is%20Valid
      (EventDispatchers|BindEventtoCogUpdatedDispatch _attachedcog (delegate Custom|Cog%20Updated))
      (EventDispatchers|BindEventtoCogSpeedChangeDispatch (Variables|Default|GetAttachedCog) (delegate Custom|CogSpeedChanged)))))