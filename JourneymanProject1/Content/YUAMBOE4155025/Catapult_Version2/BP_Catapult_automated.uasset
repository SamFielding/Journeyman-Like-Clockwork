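; Self-firing catapult that repeatedly launches a Cube projectile, starting on BeginPlay.
; A timeline swings the Handle's roll, then enables physics on the Cube and adds Charge as Y and Z velocity.
; When the Cube hits another actor, it stops simulating, the Handle resets and the timeline replays to fire again.
; The reset feeds Startpoint's world location into the Cube's relative transform.
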(event OnComponentHit(Cube)
  (params (HitComponent :type Primitive%20Component%20Object%20Reference) (OtherActor :type Actor%20Object%20Reference) (OtherComp :type Primitive%20Component%20Object%20Reference) (NormalImpulse :type Vector :default "0, 0, 0") (Hit :type Hit%20Result%20Structure%20%28by%20ref%29))
  (bind _cube (Variables|Default|GetCube))
  (bind _charge (Variables|Default|GetCharge))
  (if (!= OtherActor self)
    (Transformation|SetRelativeTransform (Variables|Default|GetCube) (Math|Transform|MakeTransform (Transformation|GetWorldLocation (Variables|Default|GetStartpoint)) "0, 0, 0" "1.000000,1.000000,1.000000") false false)
    (Physics|SetSimulatePhysics (Variables|Default|GetCube) false)
    (Transformation|SetRelativeRotation (Variables|Default|GetHandle) (Math|Rotator|MakeRotator -2e+01 0.0 0.0) false false)
    (bind _新建轨道_0 (Timeline|时间轴 PlayFromStart)
      (:Update
        (Transformation|SetWorldRotation (Variables|Default|GetHandle) (Math|Rotator|MakeRotator (Math|Float|Lerp -2e+01 3e+01 _新建轨道_0) 0.0 0.0) false false))
      (:Finished
        (Physics|SetSimulatePhysics _cube true)
        (Physics|SetPhysicsLinearVelocity _cube (Math|Vector|MakeVector 0.0 (Math|Conversions|ToFloat(Integer) _charge) (Math|Conversions|ToFloat(Integer) _charge)) true "None")))))

(event EventBeginPlay
  (bind _cube (Variables|Default|GetCube))
  (bind _charge (Variables|Default|GetCharge))
  (bind _新建轨道_0 (Timeline|时间轴 PlayFromStart)
    (:Update
      (Transformation|SetWorldRotation (Variables|Default|GetHandle) (Math|Rotator|MakeRotator (Math|Float|Lerp -2e+01 3e+01 _新建轨道_0) 0.0 0.0) false false))
    (:Finished
      (Physics|SetSimulatePhysics _cube true)
      (Physics|SetPhysicsLinearVelocity _cube (Math|Vector|MakeVector 0.0 (Math|Conversions|ToFloat(Integer) _charge) (Math|Conversions|ToFloat(Integer) _charge)) true "None"))))

(event Collision|EventActorBeginOverlap
  (params (OtherActor :type Actor%20Object%20Reference)))

(event EventTick
  (params (DeltaSeconds :type Float%20%28single-precision%29)))

(fn ConstructionScript)