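; Expandable bridge actor that extends three front and three back sections along local X when its trigger box is first overlapped.
; BeginPlay caches front and back start X positions and collapses each section onto its side's start point.
; The overlap starts six separate timelines, each lerping one section's relative X to its own endpoint.
; Helper functions change only X, preserving Y and Z; the X-scale helpers are unused.
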(event OnComponentBeginOverlap(Box)
  (params (OverlappedComponent :type Primitive%20Component%20Object%20Reference) (OtherActor :type Actor%20Object%20Reference) (OtherComp :type Primitive%20Component%20Object%20Reference) (OtherBodyIndex :type Integer) (bFromSweep :type Boolean) (SweepResult :type Hit%20Result%20Structure%20%28by%20ref%29))
  (Utilities|FlowControl|DoOnce false
    (:Completed
      (Utilities|FlowControl|Sequence
        (:then_0
          (bind _新建轨道_0 (Timeline|时间轴 Play)
            (:Update
              (bind _x (CallFunction|GetLocationX (Variables|Default|GetFront%20endpoint%201)))
              (CallFunction|SetLocaationXInprogess (Variables|Default|GetFront%20bridge%20section1) (Math|Float|Lerp (Variables|Default|GetBridgeSection_StartLocation_Front) _x _新建轨道_0)))))
        (:then_1
          (bind _新建轨道_0_2 (Timeline|Timeline Play)
            (:Update
              (bind _x_2 (CallFunction|GetLocationX (Variables|Default|GetFront%20endpoint%202)))
              (CallFunction|SetLocaationXInprogess (Variables|Default|GetFront%20bridge%20section2) (Math|Float|Lerp (Variables|Default|GetBridgeSection_StartLocation_Front) _x_2 _新建轨道_0_2)))))
        (:then_2
          (bind _新建轨道_0_3 (Timeline|Timeline_2 Play)
            (:Update
              (bind _x_3 (CallFunction|GetLocationX (Variables|Default|GetFront%20endpoint%203)))
              (CallFunction|SetLocaationXInprogess (Variables|Default|GetFront%20bridge%20section3) (Math|Float|Lerp (Variables|Default|GetBridgeSection_StartLocation_Front) _x_3 _新建轨道_0_3)))))
        (:then_3
          (bind _新建轨道_0_4 (Timeline|Timeline_0 Play)
            (:Update
              (bind _x_4 (CallFunction|GetLocationX (Variables|Default|GetBack%20endpoint1)))
              (CallFunction|SetLocaationXInprogess (Variables|Default|GetBack%20bridge%20section1) (Math|Float|Lerp (Variables|Default|GetBridgeSection_StartLocation_Back) _x_4 _新建轨道_0_4)))))
        (:then_4
          (bind _新建轨道_0_5 (Timeline|Timeline_1 Play)
            (:Update
              (bind _x_5 (CallFunction|GetLocationX (Variables|Default|GetBack%20endpoint2)))
              (CallFunction|SetLocaationXInprogess (Variables|Default|GetBack%20bridge%20section2) (Math|Float|Lerp (Variables|Default|GetBridgeSection_StartLocation_Back) _x_5 _新建轨道_0_5)))))
        (:then_5
          (bind _新建轨道_0_6 (Timeline|Timeline_3 Play)
            (:Update
              (bind _x_6 (CallFunction|GetLocationX (Variables|Default|GetBack%20endpoint3)))
              (CallFunction|SetLocaationXInprogess (Variables|Default|GetBack%20bridge%20section3) (Math|Float|Lerp (Variables|Default|GetBridgeSection_StartLocation_Back) _x_6 _新建轨道_0_6)))))))))

(event EventBeginPlay
  (Utilities|FlowControl|Sequence
    (:then_0
      (bind _x (CallFunction|GetLocationX (Variables|Default|GetFront%20startpoint%20)))
      (Variables|Default|SetBridgeSection_StartLocation_Front _x)
      (bind _x_2 (CallFunction|GetLocationX (Variables|Default|GetBack%20startpoint)))
      (Variables|Default|SetBridgeSection_StartLocation_Back _x_2))
    (:then_1
      (for _array_element (Utilities|Array|MakeArray (Variables|Default|GetFront%20bridge%20section1) (Variables|Default|GetFront%20bridge%20section2) (Variables|Default|GetFront%20bridge%20section3))
        (CallFunction|SetLocaationXStart _array_element (Variables|Default|GetFront%20startpoint%20)))
      (for _array_element_2 (Utilities|Array|MakeArray (Variables|Default|GetBack%20bridge%20section1) (Variables|Default|GetBack%20bridge%20section2) (Variables|Default|GetBack%20bridge%20section3))
        (CallFunction|SetLocaationXStart _array_element_2 (Variables|Default|GetBack%20startpoint))))))

(fn ConstructionScript)

(fn SetScaleX
  (params (目标 :type Scene%20Component%20Object%20Reference) (New%20Scale%203D%20X :type Float%20%28double-precision%29))
  (bind _relativescale3d (Variables|/Script/Engine.SceneComponent|GetRelativeScale3D 目标))
  (bind (_x _y _z) (Math|Vector|BreakVector _relativescale3d))
  (Transformation|SetRelativeScale3D 目标 (Math|Vector|MakeVector New%20Scale%203D%20X _y _z)))

(fn GetScaleX
  (params (self2 :type Scene%20Component%20Object%20Reference))
  (return (.X (Math|Vector|BreakVector (Variables|/Script/Engine.SceneComponent|GetRelativeScale3D self2)))))

(fn SetLocaationXStart
  (params (目标 :type Scene%20Component%20Object%20Reference) (startpoint :type Scene%20Component%20Object%20Reference))
  (bind _relativelocation (Variables|/Script/Engine.SceneComponent|GetRelativeLocation 目标))
  (bind (_x _y _z) (Math|Vector|BreakVector _relativelocation))
  (Transformation|SetRelativeLocation 目标 (Math|Vector|MakeVector (.X (Math|Vector|BreakVector (Variables|/Script/Engine.SceneComponent|GetRelativeLocation startpoint))) _y _z) false false))

(fn SetLocaationXInprogess
  (params (目标 :type Scene%20Component%20Object%20Reference) (New%20location :type Float%20%28double-precision%29))
  (bind _relativelocation (Variables|/Script/Engine.SceneComponent|GetRelativeLocation 目标))
  (bind (_x _y _z) (Math|Vector|BreakVector _relativelocation))
  (Transformation|SetRelativeLocation 目标 (Math|Vector|MakeVector New%20location _y _z) false false))

(fn GetLocationX
  (params (self2 :type Scene%20Component%20Object%20Reference))
  (return (.X (Math|Vector|BreakVector (Variables|/Script/Engine.SceneComponent|GetRelativeLocation self2)))))