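; Catapult actor that grabs a Character entering its sphere and flings it into the air, with power set by editor variables rather than player input.
; The overlap snaps the character to the launch point, disables movement and collision, then timelines swing the handle, launch the character and return the arm.
; Horizontal velocity comes from GetCatapultDirection with fixed upward speed; the sphere re-arms after a delay.
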(event OnComponentBeginOverlap(Sphere)
  (params (OverlappedComponent :type Primitive%20Component%20Object%20Reference) (OtherActor :type Actor%20Object%20Reference) (OtherComp :type Primitive%20Component%20Object%20Reference) (OtherBodyIndex :type Integer) (bFromSweep :type Boolean) (SweepResult :type Hit%20Result%20Structure%20%28by%20ref%29))
  ;[0.15 0.15 0.15 0.5] isPlayer?
  (bind _ascharacter (Utilities|Casting|CastToCharacter OtherActor))
  (bind _output_get (Variables|Default|SetAsCharacter _ascharacter))
  (Utilities|IsValid _output_get
    (:Is%20Valid
      (Utilities|FlowControl|Sequence
        (:then_0
          (Transformation|AttachComponentToComponent _output_get (Variables|Default|GetLaunchpoint) "None" "SnapToTarget" "SnapToTarget" "KeepRelative" false)
          (Collision|SetCollisionEnabled (Variables|Default|GetSphere) "NoCollision")
          (Utilities|FlowControl|Delay 0.2)
          (CallFunction|ThrowStart))
        (:then_1
          (Pawn|Components|CharacterMovement|DisableMovement (Variables|/Script/Engine.Character|GetCharacterMovement _output_get)))))))

(event Custom|Throw%20end
  ;[0.15 0.15 0.15 0.5] The stable version removes the feature allowing players to adjust the throwing power; instead, the power can only be changed by adjusting variables in the editor.
  (bind _新建轨道_0 (Timeline|时间轴_0 PlayFromStart)
    (:Update
      (Transformation|SetRelativeRotation (Variables|Default|GetHandle) (Math|Rotator|MakeRotator 0.0 (Math|Float|Lerp -3e+01 2e+01 _新建轨道_0) 0.0) false false))))

(event Custom|Throw%20start
  (bind (_x _y) (Utilities|GetCatapultDirection))
  (bind (_x_2 _y_2) (Utilities|GetCatapultDirection))
  (bind _launchpoint (Variables|Default|GetLaunchpoint))
  ;[0.15 0.15 0.15 0.5] The stable version removes the feature allowing players to adjust the throwing power; instead, the power can only be changed by adjusting variables in the editor.
  (Utilities|IsValid (Variables|Default|GetAsCharacter)
    (:Is%20Valid
      (bind _新建轨道_0 (Timeline|时间轴 PlayFromStart)
        (:Update
          (Transformation|SetRelativeRotation (Variables|Default|GetHandle) (Math|Rotator|MakeRotator 0.0 (Math|Float|Lerp 2e+01 -3e+01 _新建轨道_0) 0.0) false false))
        (:Finished
          (Transformation|DetachFromActor (Variables|Default|GetAsCharacter) "KeepWorld" "KeepWorld" "KeepWorld")
          (Pawn|Components|CharacterMovement|SetMovementMode (Variables|/Script/Engine.Character|GetCharacterMovement (Variables|Default|GetAsCharacter)) "MOVE_Falling" 0)
          (Character|LaunchCharacter (Variables|Default|GetAsCharacter) (Math|Vector|MakeVector _x_2 _y_2 1e+03) true true)
          (Variables|Default|SetAsCharacter 0)
          (CallFunction|ThrowEnd)
          (Utilities|FlowControl|Delay 1.0)
          (Collision|SetCollisionEnabled (Variables|Default|GetSphere) "QueryOnly"))))
    (:Is%20Not%20Valid
      (Utilities|IsValid (Variables|Default|GetOther%20Actor)
        (:Is%20Valid
          (bind _新建轨道_0_2 (Timeline|时间轴_1 PlayFromStart)
            (:Update
              (Transformation|SetRelativeRotation (Variables|Default|GetHandle) (Math|Rotator|MakeRotator 0.0 (Math|Float|Lerp 2e+01 -3e+01 _新建轨道_0_2) 0.0) false false)
              (Transformation|DetachFromActor (Variables|Default|GetOther%20Actor) "KeepWorld" "KeepWorld" "KeepWorld")
              (Class|PrimitiveComponent|AddVelocityChangeImpulseatLocation _launchpoint (Math|Vector|MakeVector _x _y 1e+03) (Variables|/Script/Engine.SceneComponent|GetRelativeLocation _launchpoint) "None")
              (Variables|Default|SetOther%20Actor 0)
              (CallFunction|ThrowEnd))))))))

(fn ConstructionScript)