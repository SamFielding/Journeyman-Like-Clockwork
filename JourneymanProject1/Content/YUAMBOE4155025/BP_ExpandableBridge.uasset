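; Expandable bridge actor that grows out when something first overlaps its trigger box.
; BeginPlay collapses all six front and back sections to zero X scale, and the box overlap fires once through a DoOnce.
; Two parallel chains of timelines then lerp each side's three sections open in sequence, the last one to half the scale of the others.
; The SetScaleX helper changes only X, preserving Y and Z.
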(event OnComponentBeginOverlap(Box)
  (params (OverlappedComponent :type Primitive%20Component%20Object%20Reference) (OtherActor :type Actor%20Object%20Reference) (OtherComp :type Primitive%20Component%20Object%20Reference) (OtherBodyIndex :type Integer) (bFromSweep :type Boolean) (SweepResult :type Hit%20Result%20Structure%20%28by%20ref%29))
  (Utilities|FlowControl|DoOnce false
    (:Completed
      (Utilities|FlowControl|Sequence
        (:then_0
          (bind _新建轨道_0 (Timeline|时间轴 Play)
            (:Update
              (CallFunction|SetScaleX (Variables|Default|GetFront%20bridge%20section1) (Math|Float|Lerp 0.0 2.0 _新建轨道_0)))
            (:Finished
              (bind _新建轨道_0_2 (Timeline|时间轴_0 Play)
                (:Update
                  (CallFunction|SetScaleX (Variables|Default|GetFront%20bridge%20section2) (Math|Float|Lerp 0.0 2.0 _新建轨道_0_2)))
                (:Finished
                  (bind _新建轨道_0_3 (Timeline|时间轴_1 Play)
                    (:Update
                      (CallFunction|SetScaleX (Variables|Default|GetFront%20bridge%20section3) (Math|Float|Lerp 0.0 1.0 _新建轨道_0_3)))))))))
        (:then_1
          (bind _新建轨道_0_4 (Timeline|时间轴_2 Play)
            (:Update
              (CallFunction|SetScaleX (Variables|Default|GetBack%20bridge%20section1) (Math|Float|Lerp 0.0 2.0 _新建轨道_0_4)))
            (:Finished
              (bind _新建轨道_0_5 (Timeline|时间轴_3 Play)
                (:Update
                  (CallFunction|SetScaleX (Variables|Default|GetBack%20bridge%20section2) (Math|Float|Lerp 0.0 2.0 _新建轨道_0_5)))
                (:Finished
                  (bind _新建轨道_0_6 (Timeline|时间轴_4 Play)
                    (:Update
                      (CallFunction|SetScaleX (Variables|Default|GetBack%20bridge%20section3) (Math|Float|Lerp 0.0 1.0 _新建轨道_0_6)))))))))))))

(event EventBeginPlay
  (for _array_element (Utilities|Array|MakeArray (Variables|Default|GetFront%20bridge%20section1) (Variables|Default|GetFront%20bridge%20section2) (Variables|Default|GetFront%20bridge%20section3) (Variables|Default|GetBack%20bridge%20section1) (Variables|Default|GetBack%20bridge%20section2) (Variables|Default|GetBack%20bridge%20section3))
    (CallFunction|SetScaleX _array_element 0.0)))

(event Collision|EventActorBeginOverlap
  (params (OtherActor :type Actor%20Object%20Reference)))

(event EventTick
  (params (DeltaSeconds :type Float%20%28single-precision%29)))

(fn ConstructionScript)

(fn SetScaleX
  (params (目标 :type Scene%20Component%20Object%20Reference) (New%20Scale%203D%20X :type Float%20%28double-precision%29))
  (bind _relativescale3d (Variables|/Script/Engine.SceneComponent|GetRelativeScale3D 目标))
  (bind (_x _y _z) (Math|Vector|BreakVector _relativescale3d))
  (Transformation|SetRelativeScale3D 目标 (Math|Vector|MakeVector New%20Scale%203D%20X _y _z)))