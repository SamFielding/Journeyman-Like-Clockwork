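; Scene component that makes its owning actor interactable, with a popup widget and an interaction box.
; On BeginPlay it adds both to the owner and attaches them to itself; overlap events show or hide the popup, which yaws toward the camera each tick.
; StartInteract passes the caller to DoInteraction.
; DestroyInteractionComponent ends the overlap before destroying children and itself, working around components that linger.
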(event EventBeginPlay
  ;[0.15 0.15 0.15 0.5] Construct Interaction Area
  (Utilities|FlowControl|Sequence
    (:then_0
      (CallFunction|ConstructWidget))
    (:then_1
      (CallFunction|ConstructCollisionBox))))

(event EventEndOverlap
  ;[0.15 0.15 0.15 0.5] Interaction Overlap Handling
  (Rendering|SetVisibility (Variables|Default|GetWidgetComponent) false false))

(event EventTick
  (params (DeltaSeconds :type Float%20%28single-precision%29))
  ;[0.15 0.15 0.15 0.5] Make Widget look at the screen
  (CallFunction|WidgetLookatCamera))

(event EventDestroyInteractionComponent
  ;[0.15 0.15 0.15 0.5] The components will, for some reason, not be destroyed properly. So, I just end the overlap and then for some reason, despite still existing they stop working. That'll do.
  (CallFunction|EndOverlap)
  (for _array_element (Components|GetChildrenComponents false)
    (Components|DestroyComponent _array_element))
  (Components|DestroyComponent))

(event EventBeginOverlap
  ;[0.15 0.15 0.15 0.5] Interaction Overlap Handling
  (Rendering|SetVisibility (Variables|Default|GetWidgetComponent) true false))

(event EventStartInteract
  (params (Caller :type KRK%20BP%20Astrobot%20Object%20Reference))
  ;[0.15 0.15 0.15 0.5] Do Interaction
  (Default|CallDoInteraction Caller))

(fn ConstructCollisionBox
  (bind _returnvalue (Game|AddComponentbyClass (Components|GetOwner) "/Script/Engine.BoxComponent" false (Variables|Default|GetInteractionBoxTransform)))
  (Variables|Default|SetInteractionBox _returnvalue)
  (Transformation|AttachComponentToComponent (Variables|Default|GetInteractionBox) self "None" "KeepRelative" "KeepRelative" "KeepRelative" true)
  (return))

(fn ConstructWidget
  (bind _returnvalue (Game|AddComponentbyClass (Components|GetOwner) "/Script/UMG.WidgetComponent" false (Variables|Default|GetInteractionPopupTransform)))
  (bind _output_get (Variables|Default|SetWidgetComponent _returnvalue))
  (UserInterface|SetWidget _output_get (Variables|Default|GetInteractionPopup))
  (Rendering|SetVisibility _output_get false true)
  (Transformation|AttachComponentToComponent (Variables|Default|GetWidgetComponent) self "None" "KeepRelative" "KeepRelative" "KeepRelative" true)
  (return))

(fn WidgetLookatCamera
  (bind _widgetcomponent (Variables|Default|GetWidgetComponent))
  (Utilities|IsValid _widgetcomponent
    (:Is%20Valid
      (if (Class|WidgetComponent|IsWidgetVisible _widgetcomponent)
        (Transformation|SetWorldRotation (Variables|Default|GetWidgetComponent) (Math|Rotator|MakeRotator 0.0 0.0 (.yaw (Math|Rotator|FindLookatRotation (Transformation|GetWorldLocation _widgetcomponent) (Camera|GetCameraLocation (Variables|/Script/Engine.PlayerController|GetPlayerCameraManager (Game|GetPlayerController 0)))))) false false)))))