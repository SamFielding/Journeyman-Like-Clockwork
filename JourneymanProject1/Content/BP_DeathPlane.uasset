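; Death plane actor that triggers respawns for falling characters that overlap it.
; On overlap with a capsule component, it checks that the actor has an AC_Checkpointer and is moving downward, then calls RespawnMessage on that component.
; A DoOnce reset on the next tick guards against duplicate triggers within a frame.
; The construction script scales the plane from the PlaneSize variable.
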(event OnComponentBeginOverlap(Plane)
  (params (OverlappedComponent :type Primitive%20Component%20Object%20Reference) (OtherActor :type Actor%20Object%20Reference) (OtherComp :type Primitive%20Component%20Object%20Reference) (OtherBodyIndex :type Integer) (bFromSweep :type Boolean) (SweepResult :type Hit%20Result%20Structure%20%28by%20ref%29))
  (bind _returnvalue (Actor|GetComponentbyClass OtherActor "/Game/AC_Checkpointer.AC_Checkpointer_C"))
  (Utilities|Casting|CastToCapsuleComponent OtherComp)
  (if (and (Utilities|IsValid _returnvalue) (< (.z (Transformation|GetVelocity OtherActor)) 0.0))
    (Utilities|FlowControl|DoOnce false :!label _label
      (:Completed
        (Class|BPICheckpointer|Respawn(Message) _returnvalue)
        (Utilities|FlowControl|DelayUntilNextTick)
        (goto _label Reset)))))

(fn ConstructionScript
  (bind _plane_size (Variables|Default|GetPlane%20Size))
  (Transformation|SetWorldScale3D (Variables|Default|GetPlane) (Math|Vector|MakeVector (/ (.x _plane_size) 1e+02) (/ (.y _plane_size) 1e+02) 1.0)))