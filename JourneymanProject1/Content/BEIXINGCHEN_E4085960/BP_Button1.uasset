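; One-shot button actor that triggers when an Astrobot overlaps its capsule during a cog roll dash.
; Three parallel timelines raise the target cog and chain, rotate the button's cog, and push the cylinder in, with start and end positions cached on BeginPlay.
; As they update, the target cog refreshes its overlaps and neighbours and CogMecanic2 is repeatedly started.
; A missing CogTarget only prints a warning at BeginPlay.
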(event OnComponentBeginOverlap(Capsule)
  (params (OverlappedComponent :type Primitive%20Component%20Object%20Reference) (OtherActor :type Actor%20Object%20Reference) (OtherComp :type Primitive%20Component%20Object%20Reference) (OtherBodyIndex :type Integer) (bFromSweep :type Boolean) (SweepResult :type Hit%20Result%20Structure%20%28by%20ref%29))
  (bind _cogtarget (Variables|Default|GetCogTarget))
  (bind _askrk_bp_astrobot (Utilities|Casting|CastToKRK_BP_Astrobot OtherActor))
  (if (Variables|/Game/BEIXINGCHEN_E4085960/BXC-CharactersSkills/BXC_AC_CogRollDash.BXC_AC_CogRollDash_C|GetIsRolling (Variables|/Game/BasicMovement/KRK_BP_Astrobot.KRK_BP_Astrobot_C|GetBXC_AC_CogRollDash _askrk_bp_astrobot))
    (Utilities|FlowControl|DoOnce false
      (:Completed
        (Utilities|FlowControl|Sequence
          (:then_0
            (bind _新建轨道_0 (Timeline|时间轴 Play)
              (:Update
                (Transformation|SetActorLocation (Variables|Default|GetCogTarget) (Math|Vector|Lerp(Vector) (Variables|Default|GetCogTargetStartLocation) (Variables|Default|GetCogTargetEndLocation) _新建轨道_0) false false)
                (Default|SetOverlappingActors _cogtarget)
                (Default|UpdateNeighbours _cogtarget)
                (Transformation|SetRelativeLocation (Variables|Default|GetWX_SM_Chains3) (Math|Vector|Lerp(Vector) (Variables|Default|GetChainStartLocation) (Variables|Default|GetChainEndLocation) _新建轨道_0) false false))))
          (:then_1
            (bind _新建轨道_0_2 (Timeline|时间轴_0 Play)
              (:Update
                (Transformation|SetRelativeRotation (Variables|Default|GetCog) (Math|Rotator|MakeRotator 0.0 _新建轨道_0_2 0.0) false false))))
          (:then_2
            (bind _新建轨道_0_3 (Timeline|时间轴_1 Play)
              (:Update
                (Transformation|SetRelativeLocation (Variables|Default|GetShape_Cylinder) (Math|Vector|Lerp(Vector) (Variables|Default|GetButtonStartLocation) (Variables|Default|GetButtonEndLocation) _新建轨道_0_3) false false)))))
        (Default|CogMecanic2Start (Variables|Default|GetCogMecanic2))))))

(event EventBeginPlay
  (bind _wx_sm_chains3 (Variables|Default|GetWX_SM_Chains3))
  (bind _shape_cylinder (Variables|Default|GetShape_Cylinder))
  (bind _cogtarget (Variables|Default|GetCogTarget))
  (bind _returnvalue (Transformation|GetActorLocation _cogtarget))
  (bind _returnvalue_2 (Transformation|GetRelativeTransform _shape_cylinder))
  (bind _returnvalue_3 (Transformation|GetRelativeTransform _wx_sm_chains3))
  (Utilities|IsValid (Variables|Default|GetCogTarget)
    (:Is%20Valid
      (Variables|Default|SetCogTargetStartLocation _returnvalue)
      (Variables|Default|SetCogTargetEndLocation (+ _returnvalue "0.000000,0.000000,400.000000"))
      (Variables|Default|SetChainStartLocation (.location _returnvalue_3))
      (Variables|Default|SetChainEndLocation (+ (.location _returnvalue_3) "0.000000,0.000000,400.000000"))
      (Variables|Default|SetButtonStartLocation (.location _returnvalue_2))
      (Variables|Default|SetButtonEndLocation (+ (.location _returnvalue_2) "0.000000,-30.000000,0.000000")))
    (:Is%20Not%20Valid
      (Development|PrintString "No target cog is selected, button will not work properly"))))

(event Collision|EventActorBeginOverlap
  (params (OtherActor :type Actor%20Object%20Reference)))

(event EventTick
  (params (DeltaSeconds :type Float%20%28single-precision%29)))

(fn ConstructionScript)