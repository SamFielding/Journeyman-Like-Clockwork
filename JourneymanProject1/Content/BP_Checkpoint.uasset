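; BP_Checkpoint is a checkpoint actor that registers a respawn-style location with any overlapping actor that has an AC_Checkpointer component.
; On overlap with its cylinder, it sends the CheckpointLocation position to that component and switches the base and head to a blue hologram material.
; Each tick, the head pivot rotates to face the last such actor.
; The OneTimeUse flag is checked but has no effect.
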(event OnComponentBeginOverlap(Cylinder)
  (params (OverlappedComponent :type Primitive%20Component%20Object%20Reference) (OtherActor :type Actor%20Object%20Reference) (OtherComp :type Primitive%20Component%20Object%20Reference) (OtherBodyIndex :type Integer) (bFromSweep :type Boolean) (SweepResult :type Hit%20Result%20Structure%20%28by%20ref%29))
  (bind _returnvalue (Actor|GetComponentbyClass OtherActor "/Game/AC_Checkpointer.AC_Checkpointer_C"))
  (Utilities|IsValid _returnvalue
    (:Is%20Valid
      (Variables|Default|SetActor OtherActor)
      (Class|BPICheckpointer|SetCheckpoint(Message) _returnvalue (Transformation|GetWorldLocation (Variables|Default|GetCheckpoint%20Location)))
      (Rendering|Material|SetMaterial (Variables|Default|Getbase) 0 "/Game/ALLARTISTS/Materials/M_Checkpoint_HoloImproved_Blue.M_Checkpoint_HoloImproved_Blue")
      (if (Variables|Default|GetOneTimeUse)
        _))))

(event EventTick
  (params (DeltaSeconds :type Float%20%28single-precision%29))
  (bind _actor (Variables|Default|GetActor))
  (bind _head_pivot (Variables|Default|Gethead%20pivot))
  (Utilities|IsValid _actor
    (:Is%20Valid
      (Transformation|SetWorldRotation _head_pivot (Math|Rotator|FindLookatRotation (Transformation|GetWorldLocation _head_pivot) (Transformation|GetActorLocation _actor)) false false))))

(fn ConstructionScript)