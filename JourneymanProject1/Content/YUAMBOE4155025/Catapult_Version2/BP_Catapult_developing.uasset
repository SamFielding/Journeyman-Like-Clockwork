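; Work-in-progress catapult that catches an overlapping Character or BP_Object on its Launchpoint and throws it when F is pressed.
; Timelines swing the Handle and return it; characters, frozen while loaded, are detached and launched when the swing finishes.
; Objects detach on the first timeline update, but the impulse targets Launchpoint rather than the object.
; Keys 1 and 2 adjust Charge, though GetCatapultDirection's Charge-scaled forward-vector math is unconnected.
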(event OnComponentBeginOverlap(Sphere)
  (params (OverlappedComponent :type Primitive%20Component%20Object%20Reference) (OtherActor :type Actor%20Object%20Reference) (OtherComp :type Primitive%20Component%20Object%20Reference) (OtherBodyIndex :type Integer) (bFromSweep :type Boolean) (SweepResult :type Hit%20Result%20Structure%20%28by%20ref%29))
  (Utilities|FlowControl|Sequence
    (:then_0
      ;[0.15 0.15 0.15 0.5] isPlayer?
      (bind _ascharacter (Utilities|Casting|CastToCharacter OtherActor))
      (bind _output_get (Variables|Default|SetAsCharacter _ascharacter))
      (Utilities|IsValid _output_get
        (:Is%20Valid
          (Utilities|FlowControl|Sequence
            (:then_0
              (Transformation|AttachComponentToComponent _output_get (Variables|Default|GetLaunchpoint) "None" "SnapToTarget" "SnapToTarget" "KeepRelative" false)
              (Collision|SetCollisionEnabled (Variables|Default|GetSphere) "NoCollision"))
            (:then_1
              (Pawn|Components|CharacterMovement|DisableMovement (Variables|/Script/Engine.Character|GetCharacterMovement _output_get)))
            (:then_2
              (Audio|PlaySound2D "/Engine/EngineSounds/1kSineTonePing.1kSineTonePing" 1.0 1.0 0.0 0 0))))))
    (:then_1
      (bind _asbp_object (Utilities|Casting|CastToBP_Object OtherActor))
      (Utilities|IsValid _asbp_object
        (:Is%20Valid
          (bind _output_get_2 (Variables|Default|SetOther%20Actor _asbp_object))
          (Transformation|AttachComponentToComponent _output_get_2 (Variables|Default|GetLaunchpoint) "None" "SnapToTarget" "SnapToTarget" "KeepRelative" false)
          (Development|PrintString (Utilities|GetDisplayName _output_get_2)))))))

(event Custom|Throw%20end
  (bind _新建轨道_0 (Timeline|时间轴_0 PlayFromStart)
    (:Update
      (Transformation|SetRelativeRotation (Variables|Default|GetHandle) (Math|Rotator|MakeRotator 0.0 (Math|Float|Lerp -3e+01 2e+01 _新建轨道_0) 0.0) false false))))

(event Custom|Throw%20start
  (bind (_x _y) (Utilities|GetCatapultDirection))
  (bind (_x_2 _y_2) (Utilities|GetCatapultDirection))
  (bind _launchpoint (Variables|Default|GetLaunchpoint))
  (Utilities|IsValid (Variables|Default|GetAsCharacter)
    (:Is%20Valid
      (bind _新建轨道_0 (Timeline|时间轴 PlayFromStart)
        (:Update
          (Transformation|SetRelativeRotation (Variables|Default|GetHandle) (Math|Rotator|MakeRotator 0.0 (Math|Float|Lerp 2e+01 -3e+01 _新建轨道_0) 0.0) false false))
        (:Finished
          (Transformation|DetachFromActor (Variables|Default|GetAsCharacter) "KeepWorld" "KeepWorld" "KeepWorld")
          (Pawn|Components|CharacterMovement|SetMovementMode (Variables|/Script/Engine.Character|GetCharacterMovement (Variables|Default|GetAsCharacter)) "MOVE_Falling" 0)
          (Character|LaunchCharacter (Variables|Default|GetAsCharacter) (Math|Vector|MakeVector _x_2 _y_2 1e+03) true true)
          (Variables|Default|SetAsCharacter 0)
          (CallFunction|ThrowEnd)
          (Utilities|FlowControl|Delay 1.0)
          (Collision|SetCollisionEnabled (Variables|Default|GetSphere) "QueryOnly"))))
    (:Is%20Not%20Valid
      (Utilities|IsValid (Variables|Default|GetOther%20Actor)
        (:Is%20Valid
          (bind _新建轨道_0_2 (Timeline|时间轴_1 PlayFromStart)
            (:Update
              (Transformation|SetRelativeRotation (Variables|Default|GetHandle) (Math|Rotator|MakeRotator 0.0 (Math|Float|Lerp 2e+01 -3e+01 _新建轨道_0_2) 0.0) false false)
              (Transformation|DetachFromActor (Variables|Default|GetOther%20Actor) "KeepWorld" "KeepWorld" "KeepWorld")
              (Class|PrimitiveComponent|AddVelocityChangeImpulseatLocation _launchpoint (Math|Vector|MakeVector _x _y 1e+03) (Variables|/Script/Engine.SceneComponent|GetRelativeLocation _launchpoint) "None")
              (Variables|Default|SetOther%20Actor 0)
              (CallFunction|ThrowEnd))))))))

(event Input|KeyboardEvents|F
  (params (Key :type Key%20Structure))
  (:Pressed
    (CallFunction|ThrowStart)))

(event Input|KeyboardEvents|1
  (params (Key :type Key%20Structure))
  (:Pressed
    (bind _output_get (Variables|Default|SetCharge (+ (Variables|Default|GetCharge) 100)))
    (Development|PrintString (Utilities|String|ToString(Integer) _output_get))))

(event Input|KeyboardEvents|2
  (params (Key :type Key%20Structure))
  (:Pressed
    (bind _output_get (Variables|Default|SetCharge (- (Variables|Default|GetCharge) 100)))
    (Development|PrintString (Utilities|String|ToString(Integer) _output_get))))

(fn ConstructionScript)