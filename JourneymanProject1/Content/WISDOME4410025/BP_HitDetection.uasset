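; BP_HitDetection is a short-lived hitbox actor that deals damage through a box overlap.
; On BeginPlay its Box copies the world transform and extent of a supplied BoxRef, if valid.
; The first overlapping actor with a WL_CPP_BASEHEALTHCOMPONENT has that component stored as EnemyRef and takes Damage, with DoOnce limiting it to a single hit.
; A Delete event destroys the actor after a given Duration.
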(event OnComponentBeginOverlap(Box)
  (params (OverlappedComponent :type Primitive%20Component%20Object%20Reference) (OtherActor :type Actor%20Object%20Reference) (OtherComp :type Primitive%20Component%20Object%20Reference) (OtherBodyIndex :type Integer) (bFromSweep :type Boolean) (SweepResult :type Hit%20Result%20Structure%20%28by%20ref%29))
  (bind _returnvalue (Actor|GetComponentbyClass OtherActor "/Script/Health.WL_CPP_BASEHEALTHCOMPONENT"))
  (Utilities|IsValid OtherActor
    (:Is%20Valid
      (Utilities|IsValid _returnvalue
        (:Is%20Valid
          (Utilities|FlowControl|DoOnce false
            (:Completed
              (Variables|Default|SetEnemyRef _returnvalue)
              (Class|WLCPPBASEHEALTHCOMPONENT|TakeDamage _returnvalue (Variables|Default|GetDamage)))))))))

(event Custom|Delete
  (params (Duration :type Float%20%28single-precision%29))
  (Utilities|FlowControl|Delay Duration)
  (Actor|DestroyActor))

(event EventBeginPlay
  (bind _boxref (Variables|Default|GetBoxRef))
  (Utilities|IsValid _boxref
    (:Is%20Valid
      (Transformation|SetWorldTransform (Variables|Default|GetBox) (Transformation|GetWorldTransform _boxref) false false)
      (Components|Box|SetBoxExtent (Variables|Default|GetBox) (Variables|/Script/Engine.BoxComponent|GetBoxExtent (Variables|Default|GetBoxRef)) true))))

(fn ConstructionScript)