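; AC_Pickup is an actor component that lets the player character pick up, drop and throw its owning actor.
; Pickup snaps the owner to the player mesh's PickUpSocket and disables its collision.
; Drop and throw detach it and restore collision, with a PickedUp flag guarding all three events.
; Throw also fires the ObjectThrown dispatcher with a scaled player forward vector, applying no force itself.
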(event Custom|ComponentPickUp
  ;[0.15 0.15 0.15 0.5] OnPickedUp
  (Development|PrintString "Pick Up is called!")
  (if (not (Variables|Default|GetPickedUp))
    (Variables|Default|SetPickedUp true)
    (Transformation|AttachComponentToComponent (Components|GetOwner) (Variables|/Script/Engine.Character|GetMesh (Game|GetPlayerCharacter 0)) "PickUpSocket" "SnapToTarget" "SnapToTarget" "SnapToTarget" true)
    (Collision|SetActorEnableCollision (Components|GetOwner) false)))

(event Custom|ComponentDrop
  ;[0.15 0.15 0.15 0.5] Drop component
  (Development|PrintString "Drop is called!")
  (if (Variables|Default|GetPickedUp)
    (Variables|Default|SetPickedUp false)
    (Transformation|DetachFromActor (Components|GetOwner) "KeepWorld" "KeepWorld" "KeepWorld")
    (Collision|SetActorEnableCollision (Components|GetOwner) true)))

(event Custom|ComponentThrow
  (if (Variables|Default|GetPickedUp)
    (Variables|Default|SetPickedUp false)
    (Transformation|DetachFromActor (Components|GetOwner) "KeepWorld" "KeepWorld" "KeepWorld")
    (Collision|SetActorEnableCollision (Components|GetOwner) true)
    (Default|CallObjectThrown (* (Transformation|GetActorForwardVector (Game|GetPlayerCharacter 0)) "1000.000000,1000.000000,1000.000000"))
    (Development|PrintString "I AM THROWING STILL")))