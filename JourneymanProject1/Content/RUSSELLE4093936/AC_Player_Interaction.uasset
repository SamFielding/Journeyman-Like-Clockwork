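; Player interaction component that detects interactable actors in front of the owning character and relays interact start and end to them.
; On BeginPlay it casts its owner and adds a forward-offset box collision at runtime.
; Overlaps message the other actor's AC_Interactable, storing the latest one and clearing it on any interactable's exit.
; StartInteract and EndInteract message the stored component, then fire InteractStarted and InteractEnded dispatchers for player-side handling.
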(event Custom|StartInteract
  ;[0.15 0.15 0.15 0.5] Updated Interact Logic
  ;;[0.15 0.15 0.15 0.5] Interact handling. Begin interaction, then call an event dispatcher to do whatever on the player.
  (Class|BPIInteraction|StartInteract(Message) (Variables|Default|GetOverlapped%20Interaction%20Component) (Variables|Default|GetPlayer))
  (Default|CallInteractStarted))

(event Custom|InteractionOverlap
  (params (OverlappedComponent :type Primitive%20Component%20Object%20Reference) (OtherActor :type Actor%20Object%20Reference) (OtherComp :type Primitive%20Component%20Object%20Reference) (OtherBodyIndex :type Integer) (bFromSweep :type Boolean) (SweepResult :type Hit%20Result%20Structure%20%28by%20ref%29))
  (bind _returnvalue (Actor|GetComponentbyClass OtherActor "/Game/RUSSELLE4093936/AC_Interactable.AC_Interactable_C"))
  ;[0.15 0.15 0.15 0.5] Overlap logic, should enable button input UI.
  (Utilities|IsValid _returnvalue
    (:Is%20Valid
      (bind _output_get (Variables|Default|SetOverlapped%20Interaction%20Component _returnvalue))
      (Class|BPIInteraction|BeginOverlap(Message) _output_get))))

(event Custom|InteractionEndOverlap
  (params (OverlappedComponent :type Primitive%20Component%20Object%20Reference) (OtherActor :type Actor%20Object%20Reference) (OtherComp :type Primitive%20Component%20Object%20Reference) (OtherBodyIndex :type Integer))
  (bind _returnvalue (Actor|GetComponentbyClass OtherActor "/Game/RUSSELLE4093936/AC_Interactable.AC_Interactable_C"))
  ;[0.15 0.15 0.15 0.5] Overlap logic, should enable button input UI.
  (Utilities|IsValid _returnvalue
    (:Is%20Valid
      (Class|BPIInteraction|EndOverlap(Message) _returnvalue)
      (Variables|Default|SetOverlapped%20Interaction%20Component 0))))

(event Custom|EndInteract
  ;[0.15 0.15 0.15 0.5] Updated Interact Logic
  ;;[0.15 0.15 0.15 0.5] On ending, call end interact regardless and handle edge-cases on the player.
  (Class|BPIInteraction|EndInteract(Message) (Variables|Default|GetOverlapped%20Interaction%20Component))
  (Default|CallInteractEnded))

(event EventBeginPlay
  ;[0.15 0.15 0.15 0.5] Create a collision area on the self, extend the collision area and bind events.
  (bind _askrk_bp_astrobot (Utilities|Casting|CastTokszdeekufhaeinaein (Components|GetOwner)))
  (bind _output_get (Variables|Default|SetPlayer _askrk_bp_astrobot))
  (bind _returnvalue (Game|AddComponentbyClass _output_get "/Script/Engine.BoxComponent" false (Math|Transform|MakeTransform "100.000000,0.000000,0.000000" "0, 0, 0" "1.000000,1.000000,1.000000")))
  (bind _output_get_2 (Variables|Default|SetInteractionArea _returnvalue))
  (Components|Box|SetBoxExtent _output_get_2 "120.000000,32.000000,85.000000" true)
  (Collision|BindEventtoOnComponentBeginOverlap (Variables|Default|GetInteractionArea) (EventDispatchers|CreateEvent :!event Custom|InteractionOverlap))
  (Collision|AssignOnComponentEndOverlap (Variables|Default|GetInteractionArea) (EventDispatchers|CreateEvent :!event Custom|InteractionEndOverlap)))