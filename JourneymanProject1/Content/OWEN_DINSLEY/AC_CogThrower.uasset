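; AC_CogThrower is a component that lets its owner throw a single cog projectile in a given direction.
; On BeginPlay it caches the owner's AC_Companion_Cog component, which it passes to each spawned cog.
; ThrowCog cycles by state: it spawns a BP_cogthrowtest at the component's location, stops that cog if moving, or despawns it if stationary.
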(event Custom|Throw%20Cog
  (params (Direction :type Vector))
  (bind _returnvalue (Components|GetOwner))
  (if (CallFunction|DoesCogExist)
    (if (Default|IsStationary (Variables|Default|GetCog%20Projectile))
      (Default|Despawn (Variables|Default|GetCog%20Projectile))
      (else
        (Default|StopMovement (Variables|Default|GetCog%20Projectile))))
    (elif (and (Utilities|IsValid _returnvalue) (Utilities|IsValid (Variables|Default|GetCompanion%20Cog)))
      (bind _returnvalue_2 (Game|SpawnActorfromClass "/Game/OWEN_DINSLEY/BP_cogthrowtest.BP_cogthrowtest_C" (Math|Conversions|ToTransform(Vector) (Transformation|GetWorldLocation)) "AlwaysSpawn" "MultiplyWithRoot" 0 (Variables|Default|GetCog%20Rotation%20Rate) Direction (Variables|Default|GetCog%20Speed) _returnvalue (Variables|Default|GetCompanion%20Cog) 0))
      (Variables|Default|SetCog%20Projectile _returnvalue_2))))

(event EventBeginPlay
  (bind _returnvalue (Components|GetOwner))
  (Utilities|IsValid _returnvalue
    (:Is%20Valid
      (Variables|Default|SetCompanion%20Cog (Actor|GetComponentbyClass _returnvalue "/Game/RUSSELLE4093936/AC_Companion_Cog.AC_Companion_Cog_C")))))

(fn DoesCogExist
  (return (Utilities|IsValid (Variables|Default|GetCog%20Projectile))))