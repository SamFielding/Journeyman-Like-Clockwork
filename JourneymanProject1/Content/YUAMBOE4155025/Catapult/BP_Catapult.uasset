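; BP_Catapult is a keyboard-controlled catapult that swings its Handle and launches a Cube projectile.
; F plays a timeline that rotates the Handle, then enables physics on the Cube and adds velocity from Charge, which keys 1 and 2 adjust.
; Hitting another actor stops Cube physics, moves it using Launchpoint's location and resets the Handle.
; Actors overlapping the Sphere are attached to Launchpoint.
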(event OnComponentHit(Cube)
  (params (HitComponent :type Primitive%20Component%20Object%20Reference) (OtherActor :type Actor%20Object%20Reference) (OtherComp :type Primitive%20Component%20Object%20Reference) (NormalImpulse :type Vector :default "0, 0, 0") (Hit :type Hit%20Result%20Structure%20%28by%20ref%29))
  (if (!= OtherActor self)
    (Transformation|SetRelativeTransform (Variables|Default|GetCube) (Math|Transform|MakeTransform (Transformation|GetWorldLocation (Variables|Default|GetLaunchpoint)) "0, 0, 0" "1.000000,1.000000,1.000000") false false)
    (Physics|SetSimulatePhysics (Variables|Default|GetCube) false)
    (Transformation|SetRelativeRotation (Variables|Default|GetHandle) (Math|Rotator|MakeRotator -2e+01 0.0 0.0) false false)))

(event OnComponentBeginOverlap(Sphere)
  (params (OverlappedComponent :type Primitive%20Component%20Object%20Reference) (OtherActor :type Actor%20Object%20Reference) (OtherComp :type Primitive%20Component%20Object%20Reference) (OtherBodyIndex :type Integer) (bFromSweep :type Boolean) (SweepResult :type Hit%20Result%20Structure%20%28by%20ref%29))
  (bind _output_get (Variables|Default|SetOther%20Actor OtherActor))
  (Transformation|AttachComponentToComponent _output_get (Variables|Default|GetLaunchpoint) "None" "SnapToTarget" "SnapToTarget" "KeepRelative" true))

(event Input|KeyboardEvents|F
  (params (Key :type Key%20Structure :default "None"))
  (bind _cube (Variables|Default|GetCube))
  (bind _charge (Variables|Default|GetCharge))
  (:Pressed
    (bind _新建轨道_0 (Timeline|时间轴 PlayFromStart)
      (:Update
        (Transformation|SetWorldRotation (Variables|Default|GetHandle) (Math|Rotator|MakeRotator (Math|Float|Lerp -2e+01 3e+01 _新建轨道_0) 0.0 0.0) false false))
      (:Finished
        (Physics|SetSimulatePhysics _cube true)
        (Physics|SetPhysicsLinearVelocity _cube (Math|Vector|MakeVector 0.0 (Math|Conversions|ToFloat(Integer) _charge) (Math|Conversions|ToFloat(Integer) _charge)) true "None")))))

(event Input|KeyboardEvents|1
  (params (Key :type Key%20Structure :default "None"))
  (:Pressed
    (bind _output_get (Variables|Default|SetCharge (+ (Variables|Default|GetCharge) 100)))
    (Development|PrintString (Utilities|String|ToString(Integer) _output_get))))

(event Input|KeyboardEvents|2
  (params (Key :type Key%20Structure :default "None"))
  (:Pressed
    (bind _output_get (Variables|Default|SetCharge (- (Variables|Default|GetCharge) 100)))
    (Development|PrintString (Utilities|String|ToString(Integer) _output_get))))

(fn ConstructionScript)