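; Player character Blueprint handling movement, camera lock-on, cog actions, HUD and pause menu.
; Inputs request combat states from a state machine, whose entry and exit events drive attack, cog throw, spin, dash and interact components, with timed resets for some.
; Move input walks and slerp-rotates the character, or spins an attached cog when movement mode is None.
; An eye-expression material function is included; the lean logic is disconnected.
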(event OnCombatStateEntries(WL_StateMachine)
  (bind _c_attack (Variables|Melee|GetC_Attack))
  ;[0.01083 0 0.5156 0.5] WISDOM-Player State Machine
  ;;[0.15 0.15 0.15 0.5] Step 2: On State Entries [START OF TRANSITION]
  (Utilities|SwitchonCombatTransition
    (:LIGHTMELEEATTACK
      (Variables|Default|SetIsAttacking true)
      (Default|LightAttack _c_attack 0.0)
      (switch int (Variables|/Game/KNOWLESE4086040/Attacks/C_Attack.C_Attack_C|GetAttack%20Stage _c_attack)
        (:0
          (Utilities|Debounce 1.0))
        (:1
          (Utilities|Debounce 1.0))
        (:2
          (Utilities|Debounce 2.0))))
    (:HEAVYMELEEATTACK
      (Default|HeavyAttack (Variables|Melee|GetC_Attack) 0.0)
      (Utilities|Debounce 0.05))
    (:COGTHROW
      (Default|ThrowCog (Variables|Default|GetAC_CogThrower) (Transformation|GetActorForwardVector (Game|GetPlayerController 0)))
      (Utilities|Debounce 2.0))
    (:COGSPIN
      (Default|OnEnterSpinAttack (Variables|CogSpin|GetBXC_AC_CogSpinAttack) 0.0))
    (:COGDASH
      (Default|OnEnterChargeDash (Variables|CogDash|GetBXC_AC_CogRollDash)))
    (:INTERACT
      (Utilities|HasCompanionCog?
        (:Empty
          (Default|StartInteract (Variables|PlayerInteraction|GetAC_Player_Interaction))
          (Utilities|Debounce 0.5))
        (:Has%20Cog
          (Utilities|IsValid (Variables|PlayerInteraction|GetAttached%20Cog)
            (:Is%20Not%20Valid
              (Default|StartInteract (Variables|PlayerInteraction|GetAC_Player_Interaction)))))))))

(event OnCombatStateExits(WL_StateMachine)
  ;[0.01083 0 0.5156 0.5] WISDOM-Player State Machine
  ;;[0.15 0.15 0.15 0.5] Step 2: On State Exits [END OF TRANSITION]
  (Utilities|SwitchonCombatTransition
    (:LIGHTMELEEATTACK
      (Variables|Default|SetIsAttacking false))
    (:COGSPIN
      (Default|OnExitSpinAttack (Variables|CogSpin|GetBXC_AC_CogSpinAttack)))
    (:COGDASH
      (Default|OnExitChargeDash (Variables|CogDash|GetBXC_AC_CogRollDash)))
    (:INTERACT
      (Utilities|HasCompanionCog?
        (:No%20Cog
          (Default|StartInteract (Variables|PlayerInteraction|GetAC_Player_Interaction)))))))

(event Custom|Move
  (bind _returnvalue (Pawn|GetControlRotation :!class /Script/Engine.Pawn))
  (bind _action_value (Variables|Default|GetAction%20Value))
  ;[0.15 0.009134 0.009134 0.502] KORUKO-Player Move Event
  (Pawn|Input|AddMovementInput (Math|Vector|GetRightVector (Math|Rotator|MakeRotator (.roll _returnvalue) 0.0 (.yaw _returnvalue))) (.x _action_value) false)
  (Pawn|Input|AddMovementInput (Math|Vector|GetForwardVector (Math|Rotator|MakeRotator 0.0 0.0 (.yaw (Pawn|GetControlRotation :!class /Script/Engine.Pawn)))) (.y _action_value) false))

(event Custom|Rotate
  (bind _action_value (Variables|Default|GetAction%20Value))
  ;[0.15 0.009134 0.009134 0.502] KORUKO-Player Rotate Event
  (Variables|Default|SetinputV3 (Math|Vector|MakeVector (.x _action_value) (.y _action_value) 0.0))
  (Transformation|SetActorRotation (Class|KismetMathLibrary|QuatRotator (Class|KismetMathLibrary|QuatSlerp (Math|Conversions|ToQuaternion(Rotator) (Transformation|GetActorRotation)) (* (Math|Conversions|ToQuaternion(Rotator) (Math|Rotator|MakeRotator 0.0 0.0 (* (.Degree2 (Utilities|Calcu)) -1.0))) (Math|Conversions|ToQuaternion(Rotator) (Variables|Default|GetOffset))) (* (Utilities|Time|GetWorldDeltaSeconds) (Variables|Default|GetRollSpeed))))))

(event Custom|Lean
  ;[0.15 0.009134 0.009134 0.502] KORUKO-Player Lean Event
  (if (not (Utilities|Enum|Equal(Enum) (Variables|/Script/Engine.CharacterMovementComponent|GetMovementMode (Variables|Character|GetCharacterMovement)) "MOVE_None"))
    (Utilities|FlowControl|Sequence
      (:then_0
        (Variables|Default|SetDeltaRotator (Math|Rotator|MakeRotator 0.0 0.0 (.yaw (Math|Rotator|Delta(Rotator) (Transformation|GetActorRotation) (Variables|Default|GetPreviousRotation)))))
        (bind _output_get (Variables|Default|SetLeanCurrent (Math|Interpolation|FInterpTo (Variables|Default|GetLeanCurrent) (Math|Float|MapRangeClamped (/ (.yaw (Variables|Default|GetDeltaRotator)) (Utilities|Time|GetWorldDeltaSeconds)) (* (Variables|Default|GetLeanPower) -1.0) (Variables|Default|GetLeanPower) -1.0 1.0) (Utilities|Time|GetWorldDeltaSeconds) 1e+01)))
        (Variables|Default|SetPreviousRotation (Transformation|GetActorRotation)))
      (:then_1
        (Transformation|SetRelativeRotation (Variables|Character|GetMesh) (Math|Rotator|MakeRotator 0.0 (.pitch (Class|KismetMathLibrary|QuatRotator (Class|KismetMathLibrary|QuatSlerp (Math|Conversions|ToQuaternion(Rotator) (Transformation|GetActorRotation)) (Math|Conversions|ToQuaternion(Rotator) (Math|Rotator|MakeRotator 0.0 (* (Variables|Default|GetLeanCurrent) (Variables|Default|GetLeanAngle)) 0.0)) (* (Utilities|Time|GetWorldDeltaSeconds) 1e+01)))) -9e+01) false false)))))

(event Input|EnhancedActionEvents|EnhancedInputActionIA_RollDash_R1
  (params (ActionValue :type Boolean) (ElapsedSeconds :type Float%20%28double-precision%29) (TriggeredSeconds :type Float%20%28double-precision%29) (InputAction :type Input%20Action%20Object%20Reference :default "/Game/BEIXINGCHEN_E4085960/BXC-CharactersSkills/IA_RollDash_R1.IA_RollDash_R1"))
  ;[0.01083 0 0.5156 0.5] WISDOM-Player State Machine
  ;;[0.15 0.15 0.15 0.5] Step 1: Input Actions and Setting State
  (:Triggered
    (Utilities|ChangeState "COGDASH"))
  (:Canceled
    (Utilities|ChangeState "RESET" :!label _label))
  (:Completed
    (goto _label)))

(event Input|EnhancedActionEvents|EnhancedInputActionKRK_IA_Move
  (params (ActionValue :type Vector%202D%20Structure) (ElapsedSeconds :type Float%20%28double-precision%29) (TriggeredSeconds :type Float%20%28double-precision%29) (InputAction :type Input%20Action%20Object%20Reference :default "/Game/Astrobot/Inputs/KRK_IA_Move.KRK_IA_Move"))
  (bind _attached_cog (Variables|PlayerInteraction|GetAttached%20Cog))
  (bind _attached_cog_2 (Variables|PlayerInteraction|GetAttached%20Cog))
  ;[0.15 0.009134 0.009134 0.502] KORUKO-Player Movement
  (:Triggered
    (bind _output_get (Variables|Default|SetAction%20Value ActionValue))
    (if (Utilities|Enum|Equal(Enum) (Variables|/Script/Engine.CharacterMovementComponent|GetMovementMode (Variables|Character|GetCharacterMovement)) "MOVE_None")
      (Utilities|IsValid _attached_cog
        (:Is%20Valid
          (CallFunction|StartSpinningCog _attached_cog (.x _output_get))))
      (else
        (Utilities|FlowControl|Sequence
          (:then_0
            (CallFunction|Move))
          (:then_1
            (if (Utilities|Enum|NotEqual(Enum) (Variables|/Script/PlayerStateMachine.StateMachineComponent|GetCurrentCombatState (Variables|StateMachine|GetWL_StateMachine)) "COGSPIN")
              (CallFunction|Rotate)))))))
  (:Canceled
    (Utilities|IsValid _attached_cog_2 :!label _label
      (:Is%20Valid
        (CallFunction|StopSpinningCog _attached_cog_2))))
  (:Completed
    (goto _label)))

(event Input|EnhancedActionEvents|EnhancedInputActionIA_Attack_Light
  (params (ActionValue :type Boolean) (ElapsedSeconds :type Float%20%28double-precision%29) (TriggeredSeconds :type Float%20%28double-precision%29) (InputAction :type Input%20Action%20Object%20Reference :default "/Game/Astrobot/Inputs/IA_Attack_Light.IA_Attack_Light"))
  ;[0.01083 0 0.5156 0.5] WISDOM-Player State Machine
  ;;[0.15 0.15 0.15 0.5] Step 1: Input Actions and Setting State
  (Utilities|ChangeState "LIGHTMELEEATTACK"))

(event Input|EnhancedActionEvents|EnhancedInputActionIA_Attack_Heavy
  (params (ActionValue :type Boolean) (ElapsedSeconds :type Float%20%28double-precision%29) (TriggeredSeconds :type Float%20%28double-precision%29) (InputAction :type Input%20Action%20Object%20Reference :default "/Game/KNOWLESE4086040/Attacks/IA_Attack_Heavy.IA_Attack_Heavy"))
  ;[0.01083 0 0.5156 0.5] WISDOM-Player State Machine
  ;;[0.15 0.15 0.15 0.5] Step 1: Input Actions and Setting State
  (Utilities|ChangeState "HEAVYMELEEATTACK"))

(event Input|EnhancedActionEvents|EnhancedInputActionIA_Spin
  (params (ActionValue :type Boolean) (ElapsedSeconds :type Float%20%28double-precision%29) (TriggeredSeconds :type Float%20%28double-precision%29) (InputAction :type Input%20Action%20Object%20Reference :default "/Game/Astrobot/Inputs/IA_Spin.IA_Spin"))
  ;[0.01083 0 0.5156 0.5] WISDOM-Player State Machine
  ;;[0.15 0.15 0.15 0.5] Step 1: Input Actions and Setting State
  (:Triggered
    (Utilities|ChangeState "COGSPIN"))
  (:Canceled
    (Utilities|ChangeState "RESET" :!label _label))
  (:Completed
    (goto _label)))

(event Input|EnhancedActionEvents|EnhancedInputActionKRK_IA_Jump
  (params (ActionValue :type Boolean) (ElapsedSeconds :type Float%20%28double-precision%29) (TriggeredSeconds :type Float%20%28double-precision%29) (InputAction :type Input%20Action%20Object%20Reference :default "/Game/Astrobot/Inputs/KRK_IA_Jump.KRK_IA_Jump"))
  ;[0.15 0.009134 0.009134 0.502] KORUKO-Player Jump - Detatch Cog From Player if Valid
  (:Started
    (Utilities|IsValid (Variables|PlayerInteraction|GetAttached%20Cog)
      (:Is%20Not%20Valid
        (Character|Jump)
        (Variables|Default|SetIsJumping true)
        (Utilities|FlowControl|Delay 0.1)
        (Variables|Default|SetIsJumping false))))
  (:Completed
    (Character|StopJumping)))

(event Input|EnhancedActionEvents|EnhancedInputActionMP_IA_CogThrow
  (params (ActionValue :type Boolean) (ElapsedSeconds :type Float%20%28double-precision%29) (TriggeredSeconds :type Float%20%28double-precision%29) (InputAction :type Input%20Action%20Object%20Reference :default "/Game/Astrobot/Inputs/MP_IA_CogThrow.MP_IA_CogThrow"))
  (bind _ac_cogthrower (Variables|Default|GetAC_CogThrower))
  ;[0.01083 0 0.5156 0.5] WISDOM-Player State Machine
  ;;[0.15 0.15 0.15 0.5] Step 1: Input Actions and Setting State
  (:Started
    (if (Default|DoesCogExist _ac_cogthrower)
      (Default|Return _ac_cogthrower)
      (else
        (Utilities|ChangeState "COGTHROW")))))

(event Input|EnhancedActionEvents|EnhancedInputActionIA_LockOn
  (params (ActionValue :type Boolean) (ElapsedSeconds :type Float%20%28double-precision%29) (TriggeredSeconds :type Float%20%28double-precision%29) (InputAction :type Input%20Action%20Object%20Reference :default "/Game/Astrobot/Inputs/IA_LockOn.IA_LockOn"))
  (bind _lockoncamera (Variables|LockOn|GetLockOnCamera))
  ;[0.15 0.08438 0 0.502] KORUKO x OWEN - Player Lock On
  (:Started
    (Class|LockonCameraComponent|LockonClosest _lockoncamera)
    (Variables|Default|SetIsLockedOn true))
  (:Completed
    (Class|LockonCameraComponent|LockOff _lockoncamera)
    (Variables|Default|SetIsLockedOn false)))

(event Input|EnhancedActionEvents|EnhancedInputActionIA_Interact
  (params (ActionValue :type Boolean) (ElapsedSeconds :type Float%20%28double-precision%29) (TriggeredSeconds :type Float%20%28double-precision%29) (InputAction :type Input%20Action%20Object%20Reference :default "/Game/BEIXINGCHEN_E4085960/BXC-CharactersSkills/IA_Interact.IA_Interact"))
  ;[0.01083 0 0.5156 0.5] WISDOM-Player State Machine
  ;;[0.15 0.15 0.15 0.5] Step 1: Input Actions and Setting State
  (Utilities|HasCompanionCog?
    (:Empty
      _)
    (:Has%20Cog
      _))
  (Utilities|IsValid (Variables|/Game/RUSSELLE4093936/AC_Player_Interaction.AC_Player_Interaction_C|GetOverlapped%20Interaction%20Component (Variables|PlayerInteraction|GetAC_Player_Interaction))
    (:Is%20Valid
      (Utilities|ChangeState "INTERACT"))))

(event Input|EnhancedActionEvents|EnhancedInputActionKRK_IA_Look
  (params (ActionValue :type Vector%202D%20Structure) (ElapsedSeconds :type Float%20%28double-precision%29) (TriggeredSeconds :type Float%20%28double-precision%29) (InputAction :type Input%20Action%20Object%20Reference :default "/Game/Astrobot/Inputs/KRK_IA_Look.KRK_IA_Look"))
  (bind (_x _y) (Math|Vector2D|BreakVector2D ActionValue))
  ;[0.15 0.08438 0 0.502] KORUKO x OWEN - Player Lock On
  (if (Variables|Default|GetIsLockedOn)
    (Class|LockonCameraComponent|SwitchTarget (Variables|LockOn|GetLockOnCamera) ActionValue)
    (else
      (Pawn|Input|AddControllerYawInput _x)
      (Pawn|Input|AddControllerPitchInput _y))))

(event Input|EnhancedActionEvents|EnhancedInputActionIA_De-Interact
  (params (ActionValue :type Boolean) (ElapsedSeconds :type Float%20%28double-precision%29) (TriggeredSeconds :type Float%20%28double-precision%29) (InputAction :type Input%20Action%20Object%20Reference :default "/Game/WISDOME4410025/IA_De-Interact.IA_De-Interact"))
  ;[0.01083 0 0.5156 0.5] WISDOM-Player State Machine
  ;;[0.15 0.15 0.15 0.5] Step 1: Input Actions and Setting State
  (Utilities|HasCompanionCog?
    (:Has%20Cog
      _)
    (:No%20Cog
      _))
  (Utilities|IsEqualto "INTERACT"
    (:true
      (Utilities|ChangeState "RESET"))))

(event Input|EnhancedActionEvents|EnhancedInputActionIA_Pause
  (params (ActionValue :type Boolean) (ElapsedSeconds :type Float%20%28double-precision%29) (TriggeredSeconds :type Float%20%28double-precision%29) (InputAction :type Input%20Action%20Object%20Reference :default "/Game/Astrobot/Inputs/IA_Pause.IA_Pause"))
  (bind _returnvalue (Game|GetPlayerController 0))
  ;[0.15 0.08438 0 0.502] KORUKO x WISDOM x KATHRYN - Player Rotation, UI Implementation
  (Input|SetInputModeUIOnly _returnvalue (Variables|UI|GetPauseMenu) "DoNotLock" false)
  (Variables|/Script/Engine.PlayerController|SetbShowMouseCursor _returnvalue true)
  (UserInterface|Viewport|AddtoViewport (Variables|UI|GetPauseMenu) 0))

(event EventHitPlayer
  ;[0.15 0.009134 0.009134 0.502] KORUKO-Player Lean and Controller Input
  (Development|PrintString "Hit"))

(event EventControllerChanged
  (params (OldController :type Controller%20Object%20Reference) (NewController :type Controller%20Object%20Reference))
  ;[0.15 0.009134 0.009134 0.502] KORUKO-Player Lean and Controller Input
  (bind _asplayer_controller (Utilities|Casting|CastToPlayerController NewController))
  (Input|AddMappingContext (PlayerController|LocalPlayerSubsystems|GetEnhancedInputLocalPlayerSubsystem _asplayer_controller) "/Game/Astrobot/Inputs/KRK_IMC_Movement.KRK_IMC_Movement" 0 "(bIgnoreAllPressedKeysUntilRelease=True,bForceImmediately=False,bNotifyUserSettings=False)"))

(event EventTick
  (params (DeltaSeconds :type Float%20%28single-precision%29))
  ;[0.15 0.009134 0.009134 0.502] KORUKO-Player Lean and Controller Input
)

(event EventBeginPlay
  (bind _returnvalue (Game|GetPlayerController 0))
  ;[0.15 0.08438 0 0.502] KORUKO x WISDOM x KATHRYN - Player Rotation, UI Implementation
  (Variables|Default|SetPreviousRotation (Transformation|GetActorRotation))
  (Utilities|FlowControl|Sequence
    (:then_0
      (bind _returnvalue_2 (UserInterface|CreateWidget "/Game/HAWESE4135711/UI/BP_HUD.BP_HUD_C" (Game|GetPlayerController 0)))
      (bind _output_get (Variables|UI|SetHUD _returnvalue_2))
      (UserInterface|Viewport|AddtoViewport _output_get 0)
      (Input|SetInputModeGameOnly _returnvalue false)
      (Variables|/Script/Engine.PlayerController|SetbShowMouseCursor _returnvalue false))
    (:then_1
      (bind _returnvalue_3 (UserInterface|CreateWidget "/Game/HAWESE4135711/UI/PauseMenu.PauseMenu_C"))
      (Variables|UI|SetPauseMenu _returnvalue_3))))

(fn ConstructionScript)

(fn EyeChange
  (params (Expression :type Integer) (Expression%20Sheet :type Float%20%28double-precision%29))
  ;[0.4062 0.02279 0] Main Eye Change System
  (Utilities|IsValid (Variables|Default|GetFace%20Param)
    (:Is%20Valid
      _)
    (:Is%20Not%20Valid
      (bind _returnvalue (Rendering|Material|CreateDynamicMaterialInstance (Variables|Character|GetMesh) 2 0 "None" :!class /Script/Engine.PrimitiveComponent))
      (Variables|Default|SetFace%20Param _returnvalue)))
  (Rendering|Material|SetScalarParameterValue (Variables|Default|GetFace%20Param) "Index" (Math|Conversions|ToFloat(Integer) Expression) :!class /Script/Engine.MaterialInstanceDynamic)
  (Rendering|Material|SetScalarParameterValue (Variables|Default|GetFace%20Param) "ExpressionSheet" Expression%20Sheet :!class /Script/Engine.MaterialInstanceDynamic))