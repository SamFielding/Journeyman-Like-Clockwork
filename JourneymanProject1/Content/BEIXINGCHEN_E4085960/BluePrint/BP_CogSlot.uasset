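; BP_CogSlot is a socket that a player character enters and spins to charge up a mechanism.
; Overlapping SlotTrigger marks the slot occupied and passes the SnapPoint transform and slot reference to the character's EnterSlot.
; SetSlopSpinning starts or stops a looping timer that accumulates clamped progress while occupied.
; Full progress stops the timer and only prints an activation placeholder; OnPlayerExit frees the slot but keeps progress.
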(event OnComponentBeginOverlap(SlotTrigger)
  (params (OverlappedComponent :type Primitive%20Component%20Object%20Reference) (OtherActor :type Actor%20Object%20Reference) (OtherComp :type Primitive%20Component%20Object%20Reference) (OtherBodyIndex :type Integer) (bFromSweep :type Boolean) (SweepResult :type Hit%20Result%20Structure%20%28by%20ref%29))
  (bind _asbp_third_person_character (Utilities|Casting|CastToBP_ThirdPersonCharacterTest OtherActor))
  (if (not (Variables|Default|GetIsPlayerInSlot))
    (bind _output_get (Variables|Default|SetCurrentPlayer _asbp_third_person_character))
    (Variables|Default|SetIsPlayerInSlot true)
    (Default|EnterSlot _output_get (Transformation|GetWorldTransform (Variables|Default|GetSnapPoint)) self)))

(event Custom|SetSlopSpinning
  (params (NewSpinning :type Boolean))
  (bind _output_get (Variables|Default|SetSlotSpinning NewSpinning))
  (if _output_get
    (bind _returnvalue (Utilities|Time|SetTimerbyEvent (delegate Custom|SlotProgressTick) (Variables|Default|GetProgressTickInterval) true))
    (Variables|Default|SetProgressTimerHandle _returnvalue)
    (else
      (Utilities|Time|ClearandInvalidateTimerbyHandle (Variables|Default|GetProgressTimerHandle)))))

(event Custom|SlotProgressTick
  (if (and (Variables|Default|GetIsPlayerInSlot) (Variables|Default|GetSlotSpinning))
    (bind _output_get (Variables|Default|SetSlotProgress (+ (Variables|Default|GetSlotProgress) (* (Variables|Default|GetProgressRatePerSecond) (Variables|Default|GetProgressTickInterval)))))
    (bind _output_get_2 (Variables|Default|SetSlotProgress (Math|Float|Clamp(Float) _output_get)))
    (if (>= _output_get_2 1.0)
      (Utilities|Time|ClearandInvalidateTimerbyHandle (Variables|Default|GetProgressTimerHandle))
      ;[0.15 0.15 0.15 0.5] Then connect the event that triggers the mechanism activation.
      (Development|PrintString "Mechanism Activated"))
    (else
      (Utilities|Time|ClearandInvalidateTimerbyHandle (Variables|Default|GetProgressTimerHandle)))))

(event Custom|OnPlayerExit
  (Variables|Default|SetIsPlayerInSlot false)
  (Variables|Default|SetCurrentPlayer 0)
  (Variables|Default|SetSlotSpinning false)
  (Utilities|Time|ClearandInvalidateTimerbyHandle (Variables|Default|GetProgressTimerHandle)))

(event EventBeginPlay)

(event Collision|EventActorBeginOverlap
  (params (OtherActor :type Actor%20Object%20Reference)))

(event EventTick
  (params (DeltaSeconds :type Float%20%28single-precision%29)))

(fn ConstructionScript)