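; BP_AutoDoor is a door actor that moves vertically in response to a cog system through its ACCogListener component.
; Cog state updates enable the door only for one specific state, and speed updates store the current speed.
; Each speed update while enabled restarts the DoorMovement timeline, whose updates add Height, scaled by speed clamped to ±1, onto the actor's current Z, so movement accumulates and its direction follows the speed's sign.
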(event Custom|Cog%20Updated
  (params (State :type E_State%20Enum :default "NewEnumerator0"))
  (if (Utilities|Enum|Equal(Enum) State "NewEnumerator3")
    (Variables|Default|SetIs%20Enabled true)
    (else
      (Variables|Default|SetIs%20Enabled false))))

(event Custom|Cog%20Speed%20Updated
  (params (Speed :type Float%20%28double-precision%29))
  (bind _returnvalue (Transformation|GetActorTransform))
  (bind _output_get (Variables|Default|SetCurrentSpeed Speed))
  (if (Variables|Default|GetIs%20Enabled)
    (bind _height (Timeline|DoorMovement PlayFromStart)
      (:Update
        (Transformation|SetActorRelativeLocation (Math|Vector|MakeVector (.x (.location _returnvalue)) (.y (.location _returnvalue)) (+ (.z (.location _returnvalue)) (* (* _height 1.0) (Math|Float|Clamp(Float) _output_get -1.0)))))))))

(event EventBeginPlay
  (bind _ac_cog_listener (Variables|Default|GetAC_Cog_Listener))
  ;[0.15 0.15 0.15 0.5] Events
  (EventDispatchers|BindEventtoCogUpdated _ac_cog_listener (EventDispatchers|CreateEvent :!event Custom|Cog%20Updated))
  (EventDispatchers|BindEventtoCogSpeedUpdated _ac_cog_listener (EventDispatchers|CreateEvent :!event Custom|Cog%20Speed%20Updated)))

(fn ConstructionScript)